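; BP_ToonSky is a sky Blueprint that passes the sun direction to the toon sky's Material Parameter Collection.
; UpdateSunDirection writes the forward vector of the referenced directional light actor into the LightVector parameter of MPC_ToonSky.
; It runs at BeginPlay and in the Construction Script, with a self-resetting RefreshMaterial bool acting as an editor refresh button.
; There is no per-frame update.
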(event EventBeginPlay
  (CallFunction|UpdateSunDirection))

(event Collision|EventActorBeginOverlap
  (params (OtherActor :type Actor%20Object%20Reference)))

(event EventTick
  (params (DeltaSeconds :type Float%20%28single-precision%29)))

(fn ConstructionScript
  (if (Variables|Default|GetRefresh%20material) ; Updating bool in details panel causes construction script to run again
    _
    (else
      _))
  (Variables|Default|SetRefresh%20material false)
  (CallFunction|UpdateSunDirection))

(fn UpdateSunDirection
  (Rendering|Material|SetVectorParameterValue "/Game/Environment/Sky/Materials/MPC_ToonSky.MPC_ToonSky" "LightVector" (Math|Conversions|ToLinearColor(Vector) (Math|Rotator|GetRotationXVector (Transformation|GetActorRotation (Variables|Default|GetDirectional%20light%20actor)))) :!class /Script/Engine.KismetMaterialLibrary))