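; BP_Stun is a stun buff for units in the turn-based JRPG template.
; Applying the buff sets the target unit's IsStun flag and plays that unit's stun montage.
; When the buff ends, it clears the flag and plays the unit's idle montage.
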(event EventApplyBuff
  (bind _targetunit (Variables|Default|GettargetUnit))
  (Variables|/Game/TurnBasedJRPGTemplate/Blueprints/Units/BP_UnitBase.BP_UnitBase_C|SetisStun _targetunit true)
  (Default|PlayAnimationMontage _targetunit (Variables|/Game/TurnBasedJRPGTemplate/Blueprints/Units/BP_UnitBase.BP_UnitBase_C|GetstunAnimationMontage _targetunit)))

(event EventOnBuffEnded
  (bind _targetunit (Variables|Default|GettargetUnit))
  (Variables|/Game/TurnBasedJRPGTemplate/Blueprints/Units/BP_UnitBase.BP_UnitBase_C|SetisStun _targetunit false)
  (Default|PlayAnimationMontage _targetunit (Variables|/Game/TurnBasedJRPGTemplate/Blueprints/Units/BP_UnitBase.BP_UnitBase_C|GetIdleAnimationMontage _targetunit)))

(fn ConstructionScript
  (|CallParentFunction))