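; Overworld player pawn for Vahn in the turn-based JRPG template, with hard-wired runtime equipment swapping.
; Keys 1 and 2 switch the Chest mesh between Starter and Hunter sets, and keys 3 and 4 do the same for Legs.
; Each swap keeps the current pose and sets ABP_Vahn as the anim class on that component.
; Construction only calls the parent, and some disconnected pose-reinit swap nodes never run.
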(event OnConstraintBroken(Mesh)
  (params (ConstraintIndex :type Integer)))

(event Input|KeyboardEvents|8
  (params (Key :type Key%20Structure))
  ;[1 1 1] Vehicle Swapping @Runtime
)

(event Input|KeyboardEvents|9
  (params (Key :type Key%20Structure))
  ;[1 1 1] Vehicle Swapping @Runtime
)

(event Input|KeyboardEvents|1
  (params (Key :type Key%20Structure))
  (bind _chest (Variables|Default|GetChest))
  ;[1 1 1] Vehicle Swapping @Runtime
  (:Pressed
    (Class|SkinnedMeshComponent|SetSkeletalMesh _chest "/Game/OurStuff/Characters/Vahn/Equipment/BasicOutfit/EQ_Vahn_Chest_Starter.EQ_Vahn_Chest_Starter" false)
    (Class|SkeletalMeshComponent|SetAnimClass _chest "/Game/OurStuff/Characters/Vahn/ABP_Vahn.ABP_Vahn_C")))

(event Input|KeyboardEvents|0
  (params (Key :type Key%20Structure))
  ;[1 1 1] Vehicle Swapping @Runtime
)

(event Input|KeyboardEvents|2
  (params (Key :type Key%20Structure))
  (bind _chest (Variables|Default|GetChest))
  ;[1 1 1] Vehicle Swapping @Runtime
  (:Pressed
    (Class|SkinnedMeshComponent|SetSkeletalMesh _chest "/Game/OurStuff/Characters/Vahn/Equipment/HunterClothes/EQ_Vahn_Chest_Hunter.EQ_Vahn_Chest_Hunter" false)
    (Class|SkeletalMeshComponent|SetAnimClass _chest "/Game/OurStuff/Characters/Vahn/ABP_Vahn.ABP_Vahn_C")))

(event Input|KeyboardEvents|3
  (params (Key :type Key%20Structure))
  (bind _legs (Variables|Default|GetLegs))
  ;[1 1 1] Vehicle Swapping @Runtime
  (:Pressed
    (Class|SkinnedMeshComponent|SetSkeletalMesh _legs "/Game/OurStuff/Characters/Vahn/Equipment/BasicOutfit/EQ_Vahn_Legs_Starter.EQ_Vahn_Legs_Starter" false)
    (Class|SkeletalMeshComponent|SetAnimClass _legs "/Game/OurStuff/Characters/Vahn/ABP_Vahn.ABP_Vahn_C")))

(event Input|KeyboardEvents|4
  (params (Key :type Key%20Structure))
  (bind _legs (Variables|Default|GetLegs))
  ;[1 1 1] Vehicle Swapping @Runtime
  (:Pressed
    (Class|SkinnedMeshComponent|SetSkeletalMesh _legs "/Game/OurStuff/Characters/Vahn/Equipment/HunterClothes/EQ_Vahn_Legs_Hunter.EQ_Vahn_Legs_Hunter" false)
    (Class|SkeletalMeshComponent|SetAnimClass _legs "/Game/OurStuff/Characters/Vahn/ABP_Vahn.ABP_Vahn_C")))

(event Input|KeyboardEvents|5
  (params (Key :type Key%20Structure))
  ;[1 1 1] Vehicle Swapping @Runtime
)

(event Input|KeyboardEvents|6
  (params (Key :type Key%20Structure))
  ;[1 1 1] Vehicle Swapping @Runtime
)

(event Input|KeyboardEvents|7
  (params (Key :type Key%20Structure))
  ;[1 1 1] Vehicle Swapping @Runtime
)

(fn ConstructionScript
  (|CallParentFunction))